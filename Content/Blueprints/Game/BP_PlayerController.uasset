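; Player controller that turns Enhanced Input move, look, jump and sprint actions into calls on the cached BP_Player.
; Look input is smoothed with FInterpTo, and movement follows the control rotation.
; Head-bob camera shakes switch between idle, walking and running based on the character's movement state, with bindings to its initialization and speed-change events.
; It also relays hitmarker and tutorial-panel toggles to BP_HUD.
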(event Custom|ShowHitmarker
  ;[0.15 0.15 0.15 0.5] Notify HUD to display hitmarker
  (bind _asbp_hud (Utilities|Casting|CastToBP_HUD (HUD|GetHUD)))
  (Default|ShowHitmarker _asbp_hud))

(event EventBeginPlay
  (CallFunction|CachePlayerCharacter)
  (CallFunction|BindEvents))

(event Input|EnhancedActionEvents|EnhancedInputActionIA_Move
  (params (ActionValue :type Vector%202D%20Structure) (ElapsedSeconds :type Float%20%28double-precision%29) (TriggeredSeconds :type Float%20%28double-precision%29) (InputAction :type Input%20Action%20Object%20Reference :default "/Game/Input/Actions/IA_Move.IA_Move"))
  ;[0.15 0.1139 0.009679 0.5] Movement
  (:Triggered
    (Movement|MoveLeftRight (.x ActionValue))
    (Movement|MoveForwardBackward (.y ActionValue)))
  (:Completed
    (Default|SetMovementState (Variables|Default|GetPlayerCharacter) false)
    (Movement|ShakeCamera)))

(event Input|EnhancedActionEvents|EnhancedInputActionIA_Look
  (params (ActionValue :type Vector%202D%20Structure) (ElapsedSeconds :type Float%20%28double-precision%29) (TriggeredSeconds :type Float%20%28double-precision%29) (InputAction :type Input%20Action%20Object%20Reference :default "/Game/Input/Actions/IA_Look.IA_Look"))
  ;[0.15 0.1139 0.009679 0.5] Movement
  (Movement|LookLeftRight (.x ActionValue))
  (Movement|LookUpDown (.y ActionValue)))

(event Input|EnhancedActionEvents|EnhancedInputActionIA_Jump
  (params (ActionValue :type Boolean) (ElapsedSeconds :type Float%20%28double-precision%29) (TriggeredSeconds :type Float%20%28double-precision%29) (InputAction :type Input%20Action%20Object%20Reference :default "/Game/Input/Actions/IA_Jump.IA_Jump"))
  ;[0.15 0.1139 0.009679 0.5] Movement
  (:Started
    (Character|Jump (Variables|Default|GetPlayerCharacter))))

(event Input|EnhancedActionEvents|EnhancedInputActionIA_Sprint
  (params (ActionValue :type Boolean) (ElapsedSeconds :type Float%20%28double-precision%29) (TriggeredSeconds :type Float%20%28double-precision%29) (InputAction :type Input%20Action%20Object%20Reference :default "/Game/Input/Actions/IA_Sprint.IA_Sprint"))
  ;[0.15 0.1139 0.009679 0.5] Movement
  (:Started
    (Default|ToogleRunning (Variables|Default|GetPlayerCharacter) true))
  (:Completed
    (Default|ToogleRunning (Variables|Default|GetPlayerCharacter) false)))

(event Input|EnhancedActionEvents|EnhancedInputActionIA_TutorialPanel
  (params (ActionValue :type Boolean) (ElapsedSeconds :type Float%20%28double-precision%29) (TriggeredSeconds :type Float%20%28double-precision%29) (InputAction :type Input%20Action%20Object%20Reference :default "/Game/Input/Actions/IA_TutorialPanel.IA_TutorialPanel"))
  (:Started
    (bind _asbp_hud (Utilities|Casting|CastToBP_HUD (HUD|GetHUD)))
    (Default|ToggleTutorialPanel _asbp_hud)))

(event Custom|BindEvents
  (EventDispatchers|BindEventtoOnCharacterInitialization (Variables|Default|GetPlayerCharacter) (EventDispatchers|CreateEvent :!event Custom|OnCharacterInit))
  (EventDispatchers|BindEventtoOnChangeSpeed (Variables|Default|GetPlayerCharacter) (EventDispatchers|CreateEvent :!event Custom|ChangeCameraClass)))

(event Custom|ChangeCameraClass
  (Movement|AdjustCameraShake))

(event Custom|OnCharacterInit
  (Movement|ShakeCamera))

(fn ConstructionScript)

(fn CachePlayerCharacter
  (bind _asbp_player (Utilities|Casting|CastToBP_Player (Game|GetPlayerCharacter 0)))
  (Variables|Default|SetPlayerCharacter _asbp_player)
  (return))

(fn ShakeCamera
  (if (Variables|/Game/Blueprints/Characters/Player/BP_Player.BP_Player_C|GetIsMoving (Variables|Default|GetPlayerCharacter))
    (bind _returnvalue (CameraShakes|StartCameraShake (Game|GetPlayerCameraManager 0) (Variables|Movement|GetCameraShakeClass) (Variables|Movement|GetCameraShakeScale) "CameraLocal" "0, 0, 0"))
    (Variables|Movement|SetShakeInstance _returnvalue)
    (return)
    (else
      (CameraShakes|StopCameraShake (Game|GetPlayerCameraManager 0) (Variables|Movement|GetShakeInstance) false)
      (bind _returnvalue_2 (CameraShakes|StartCameraShake (Game|GetPlayerCameraManager 0) "/Game/Blueprints/Misc/CameraShake/CamShake_HeadBob_Idle.CamShake_HeadBob_Idle_C" 1.0 "CameraLocal" "0, 0, 0"))
      (Variables|Movement|SetShakeInstance _returnvalue_2)
      (return))))

(fn MoveForwardBackward
  (params (ValueY :type Float%20%28double-precision%29))
  (Default|SetMovementState (Variables|Default|GetPlayerCharacter) true)
  (Pawn|Input|AddMovementInput (Variables|Default|GetPlayerCharacter) (Math|Vector|GetForwardVector (Pawn|GetControlRotation :!class /Script/Engine.Controller)) ValueY false)
  (Movement|ShakeCamera)
  (return))

(fn MoveLeftRight
  (params (ValueX :type Float%20%28double-precision%29))
  (Default|SetMovementState (Variables|Default|GetPlayerCharacter) true)
  (Pawn|Input|AddMovementInput (Variables|Default|GetPlayerCharacter) (Math|Vector|GetRightVector (Pawn|GetControlRotation :!class /Script/Engine.Controller)) ValueX false)
  (Movement|ShakeCamera)
  (return))

(fn LookLeftRight
  (params (ValueX :type Float%20%28double-precision%29))
  (bind _output_get (Variables|Movement|SetInputAxisLookX (Math|Interpolation|FInterpTo (Variables|Movement|GetInputAxisLookX) ValueX (Utilities|Time|GetWorldDeltaSeconds) 9e+01)))
  (Pawn|Input|AddControllerYawInput (Variables|Default|GetPlayerCharacter) _output_get)
  (return))

(fn LookUpDown
  (params (ValueY :type Float%20%28double-precision%29))
  (bind _output_get (Variables|Movement|SetInputAxisLookY (Math|Interpolation|FInterpTo (Variables|Movement|GetInputAxisLookY) ValueY (Utilities|Time|GetWorldDeltaSeconds) 9e+01)))
  (Pawn|Input|AddControllerPitchInput (Variables|Default|GetPlayerCharacter) _output_get)
  (return))

(fn ChangeShakeCamera
  (params (CameraShakeClass :type Camera%20Shake%20Base%20Class%20Reference) (CameraShakeScale :type Float%20%28single-precision%29))
  (Variables|Movement|SetCameraShakeClass CameraShakeClass)
  (Variables|Movement|SetCameraShakeScale CameraShakeScale)
  (return))

(fn AdjustCameraShake
  (CameraShakes|StopCameraShake (Game|GetPlayerCameraManager 0) (Variables|Movement|GetShakeInstance) false)
  (if (Variables|/Game/Blueprints/Characters/Player/BP_Player.BP_Player_C|GetIsRunning (Variables|Default|GetPlayerCharacter))
    (Movement|ChangeShakeCamera "/Game/Blueprints/Misc/CameraShake/CamShake_HeadBob_Running.CamShake_HeadBob_Running_C" 1.0)
    (else
      (Movement|ChangeShakeCamera "/Game/Blueprints/Misc/CameraShake/CamShake_HeadBob_Walking.CamShake_HeadBob_Walking_C" 0.7)
      (if (not (Variables|/Game/Blueprints/Characters/Player/BP_Player.BP_Player_C|GetIsMoving (Variables|Default|GetPlayerCharacter)))
        (Movement|ChangeShakeCamera "/Game/Blueprints/Misc/CameraShake/CamShake_HeadBob_Idle.CamShake_HeadBob_Idle_C" 1.0)))))