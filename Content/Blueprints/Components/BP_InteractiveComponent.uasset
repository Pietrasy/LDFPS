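; Actor component that lets its owning Character interact with nearby objects on input.
; On BeginPlay it caches the owner and binds to its capsule's begin and end overlap events.
; Overlapping actors that implement BPI_Interactable are tracked in an Interactables array.
; The IA_Interact Enhanced Input action sends InteractMessage, with the owner character, to the last entry in that array if valid.
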(event Custom|HandleBeginOverlap
  (params (OverlappedComponent :type Primitive%20Component%20Object%20Reference) (OtherActor :type Actor%20Object%20Reference) (OtherComp :type Primitive%20Component%20Object%20Reference) (OtherBodyIndex :type Integer) (bFromSweep :type Boolean) (SweepResult :type Hit%20Result%20Structure%20%28by%20ref%29))
  (if (Utilities|DoesObjectImplementInterface OtherActor "/Game/Blueprints/Interfaces/BPI_Interactable.BPI_Interactable_C")
    (Utilities|Array|Add (Variables|Default|GetInteractables) OtherActor)))

(event Custom|HandleEndOverlap
  (params (OverlappedComponent :type Primitive%20Component%20Object%20Reference) (OtherActor :type Actor%20Object%20Reference) (OtherComp :type Primitive%20Component%20Object%20Reference) (OtherBodyIndex :type Integer))
  (if (Utilities|DoesObjectImplementInterface OtherActor "/Game/Blueprints/Interfaces/BPI_Interactable.BPI_Interactable_C")
    (Utilities|Array|RemoveItem (Variables|Default|GetInteractables) OtherActor)))

(event Input|EnhancedActionEvents|EnhancedInputActionIA_Interact
  (params (ActionValue :type Boolean) (ElapsedSeconds :type Float%20%28double-precision%29) (TriggeredSeconds :type Float%20%28double-precision%29) (InputAction :type Input%20Action%20Object%20Reference :default "/Game/Input/Actions/IA_Interact.IA_Interact"))
  (:Started
    (bind _interactable (CallFunction|GetInteractable))
    (Utilities|IsValid _interactable
      (:Is%20Valid
        (Class|BPIInteractable|Interact(Message) _interactable (Variables|Default|GetOwnerCharacter))))))

(event EventBeginPlay
  (CallFunction|CacheOwnerCharacter)
  (Collision|BindEventtoOnComponentBeginOverlap (Variables|/Script/Engine.Character|GetCapsuleComponent (Variables|Default|GetOwnerCharacter)) (EventDispatchers|CreateEvent :!event Custom|HandleBeginOverlap))
  (Collision|BindEventtoOnComponentEndOverlap (Variables|/Script/Engine.Character|GetCapsuleComponent (Variables|Default|GetOwnerCharacter)) (EventDispatchers|CreateEvent :!event Custom|HandleEndOverlap)))

(fn CacheOwnerCharacter
  (bind _ascharacter (Utilities|Casting|CastToCharacter (Components|GetOwner)))
  (Variables|Default|SetOwnerCharacter _ascharacter)
  (return))

(fn GetInteractable
  (if (Utilities|Array|IsNotEmpty (Variables|Default|GetInteractables))
    (return (Utilities|Array|Get(acopy) (Variables|Default|GetInteractables) (Utilities|Array|LastIndex (Variables|Default|GetInteractables))))))