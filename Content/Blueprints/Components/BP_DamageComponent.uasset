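; Actor component that reacts whenever its owning actor takes damage, giving hit feedback.
; On BeginPlay it caches the owner and binds to its point, radial and any damage events.
; All three handlers funnel into RespondToDamage, which shows a hitmarker message on the first player's HUD and broadcasts OnTakeDamage.
; Damage details are not passed on, and no health is tracked here.
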(event Custom|HandlePointDamage
  (params (DamagedActor :type Actor%20Object%20Reference) (Damage :type Float%20%28single-precision%29) (InstigatedBy :type Controller%20Object%20Reference) (HitLocation :type Vector) (FHitComponent :type Primitive%20Component%20Object%20Reference) (BoneName :type Name) (ShotFromDirection :type Vector) (DamageType :type Damage%20Type%20Object%20Reference) (DamageCauser :type Actor%20Object%20Reference))
  (CallFunction|RespondtoDamage))

(event Custom|HandleRadialDamage
  (params (DamagedActor :type Actor%20Object%20Reference) (Damage :type Float%20%28single-precision%29) (DamageType :type Damage%20Type%20Object%20Reference) (Origin :type Vector) (HitInfo :type Hit%20Result%20Structure%20%28by%20ref%29) (InstigatedBy :type Controller%20Object%20Reference) (DamageCauser :type Actor%20Object%20Reference))
  (CallFunction|RespondtoDamage))

(event Custom|HandleAnyDamage
  (params (DamagedActor :type Actor%20Object%20Reference) (Damage :type Float%20%28single-precision%29) (DamageType :type Damage%20Type%20Object%20Reference) (InstigatedBy :type Controller%20Object%20Reference) (DamageCauser :type Actor%20Object%20Reference))
  (CallFunction|RespondtoDamage))

(event EventBeginPlay
  (CallFunction|CacheOwner)
  (EventDispatchers|BindEventtoOnTakePointDamage (Variables|Default|GetOwner) (EventDispatchers|CreateEvent :!event Custom|HandlePointDamage))
  (EventDispatchers|BindEventtoOnTakeRadialDamage (Variables|Default|GetOwner) (EventDispatchers|CreateEvent :!event Custom|HandleRadialDamage))
  (EventDispatchers|BindEventtoOnTakeAnyDamage (Variables|Default|GetOwner) (EventDispatchers|CreateEvent :!event Custom|HandleAnyDamage)))

(fn CacheOwner
  (Variables|Default|SetOwner (Components|GetOwner))
  (return))

(fn RespondtoDamage
  (Class|BPIHUD|ShowHitmarker(Message) (HUD|GetHUD (Game|GetPlayerController 0)))
  (Default|CallOnTakeDamage)
  (return))