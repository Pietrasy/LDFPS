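; BP_ExplosiveBarrel is a barrel actor that explodes shortly after taking any damage.
; The damage event stores the instigating controller, disables further damage and starts a short randomized timer that calls Explosion, staggering chain reactions.
; Explosion applies full radial damage credited to that instigator on the Destructible prevention channel, spawns attenuated sound and a particle system, then destroys the actor.
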(event Game|Damage|EventAnyDamage
  (params (Damage :type Float%20%28single-precision%29) (DamageType :type Damage%20Type%20Object%20Reference) (InstigatedBy :type Controller%20Object%20Reference) (DamageCauser :type Actor%20Object%20Reference))
  (Variables|Default|SetDamageInstigator InstigatedBy)
  (Variables|Actor|SetbCanBeDamaged false)
  (bind _returnvalue (Utilities|Time|SetTimerbyFunctionName 0 "Explosion" (Math|Random|RandomFloatinRange 0.05 0.15)))
  (Variables|Default|SetExplosion_TimerHandle _returnvalue))

(fn ConstructionScript)

(fn Explosion
  (bind _returnvalue (Transformation|GetActorTransform))
  (Game|Damage|ApplyRadialDamage (Variables|Default|GetExplosionDamage) (Transformation|GetActorLocation) 4e+02 "/Script/Engine.DamageType" 0 self (Variables|Default|GetDamageInstigator) true "ECC_Destructible")
  (Audio|SpawnSoundatLocation (Variables|Default|GetExplosionSound) (Transformation|GetActorLocation) "0, 0, 0" 1.0 1.0 0.0 "/Game/Art/Audio/Explosion/ATT_Explosions.ATT_Explosions" 0)
  (Niagara|SpawnSystematLocation (Variables|Default|GetExplosionParticle) (.location _returnvalue) (.rotation _returnvalue) (.scale _returnvalue))
  (Actor|DestroyActor)
  (return))