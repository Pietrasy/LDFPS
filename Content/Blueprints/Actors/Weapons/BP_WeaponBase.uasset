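; Base weapon actor driven by WeaponData, handling full-auto, single and burst fire, ammo, recoil and reload.
; Timers and DoN/DoOnce gates pace fire modes and lock shots between rounds.
; Each shot line-traces with random spread to apply point damage, then spawns a projectile toward the result, with timeline-driven recoil and muzzle light.
; Reload spins the weapon on a timeline before refilling ammo; dispatcher calls report shots and ammo updates.
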(event Custom|OnReload
  ;[0.15 0.15 0.15 0.5] Reload animation
  (if (Variables|Default|GetIsEnable)
    (Variables|Reload|SetPreviousRotation 0.0)
    (bind _interpolation (Timeline|Reload_Timeline PlayFromStart)
      (:Update
        (Utilities|RotateWeapon _interpolation))
      (:Finished
        (Ammo|SetAmmoCount (Variables|/Game/Blueprints/Data/DataAssets/Weapons/PDA_WeaponData.PDA_WeaponData_C|GetMaxAmmo (Variables|Default|GetWeaponData)))
        (WeaponManagment|EnableWeapon))
      (:PlayReloadSound
        (Sound|PlayReloadSound)))))

(event Custom|EndShot
  ;[0.15 0.15 0.15 0.5] Fire states
  (CallFunction|LockFire)
  (Timers|SetTimerforUnlockFire false)
  (WeaponManagment|UpdateWeapon))

(event Custom|StartFire
  ;[0.15 0.15 0.15 0.5] Handles fire modes
  (if (Variables|Parameters|GetCanFire)
    (switch Utilities|FlowControl|Switch|SwitchonEFireMode (Variables|/Game/Blueprints/Data/DataAssets/Weapons/PDA_WeaponData.PDA_WeaponData_C|GetFireMode (Variables|Default|GetWeaponData))
      (:NewEnumerator0
        (Firing|Fire))
      (:NewEnumerator1
        (Utilities|FlowControl|DoN 1
          (:Exit
            (Firing|Fire))))
      (:NewEnumerator2
        (if (not (Utilities|Time|IsTimerActivebyHandle (Variables|Timers|GetStartBurstMode_TimerHandle)))
          (Timers|SetTimerforStartBurstMode)
          (CallFunction|StartBurstMode))))))

(event Custom|ApplyRecoil
  ;[0.15 0.15 0.15 0.5] Recoil
  (bind (_direction _recoilinterpolation) (Timeline|RecoilMovement_Timeline Play)
    (:Update
      (Firing|CalcutateRecoil _direction _recoilinterpolation))
    (:Finished
      (Utilities|String|Reverse (Variables|Default|GetRecoilMovement_Timeline)))))

(event Custom|ShowMuzzleLight
  ;[0.15 0.15 0.15 0.5] Set alpha muzzle light
  (Rendering|SetVisibility (Variables|Default|GetMuzzleLight) true false)
  (bind _alpha (Timeline|MuzzleLight_Timeline PlayFromStart)
    (:Update
      (Rendering|Components|Light|SetIntensity (Variables|Default|GetMuzzleLight) (Math|Float|Lerp 4e+02 0.0 _alpha)))
    (:Finished
      (Rendering|SetVisibility (Variables|Default|GetMuzzleLight) false false))))

(event Custom|UnlockSingleMode
  ;[0.15 0.15 0.15 0.5] Handles fire modes
  (Utilities|FlowControl|DoN 1) ; enters at Reset
)

(event Custom|LockFire
  ;[0.15 0.15 0.15 0.5] Fire states
  (Variables|Parameters|SetCanFire false))

(event Custom|StartBurstMode
  ;[0.15 0.15 0.15 0.5] Burst mode
  (Utilities|FlowControl|DoOnce false
    (:Completed
      (CallFunction|BurstMode))))

(event Custom|BurstMode
  ;[0.15 0.15 0.15 0.5] Burst mode
  (bind _counter (Utilities|FlowControl|DoN 3)
    (:Exit
      (Firing|Fire)
      (if (== _counter 3)
        (Timers|SetTimerforUnlockBurstMode)))))

(event Custom|UnlockFire
  ;[0.15 0.15 0.15 0.5] Fire states
  (Variables|Parameters|SetCanFire true)
  (Audio|Components|Audio|Stop (Variables|Default|GetRecoilMovement_Timeline)))

(event Custom|OnDisableWeapon
  ;[0.15 0.15 0.15 0.5] Weapon states
  (CallFunction|LockFire)
  (CallFunction|UnlockSingleMode)
  (CallFunction|UnlockBurstMode)
  (Rendering|SetVisibility (Variables|Default|GetMuzzleLight) false false))

(event Custom|UnlockBurstMode
  ;[0.15 0.15 0.15 0.5] Burst mode
  (Utilities|Time|ClearandInvalidateTimerbyHandle (Variables|Timers|GetStartBurstMode_TimerHandle))
  (Utilities|FlowControl|Sequence
    (:then_0
      (Utilities|FlowControl|DoOnce false) ; enters at Reset
    )
    (:then_1
      (Utilities|FlowControl|DoN 3) ; enters at Reset
    )))

(event Custom|OnEnableWeapon
  ;[0.15 0.15 0.15 0.5] Weapon states
  (Timers|SetTimerforUnlockFire true))

(fn ConstructionScript)

(fn SetAmmoCount
  (params (NewAmmoCount :type Integer))
  (Variables|Parameters|SetCurrentAmmo (Math|Integer|Clamp(Integer) NewAmmoCount 0 (Variables|/Game/Blueprints/Data/DataAssets/Weapons/PDA_WeaponData.PDA_WeaponData_C|GetMaxAmmo (Variables|Default|GetWeaponData))))
  (return))

(fn SpreadBullet
  (params (FireLine :type Vector))
  (bind (_x _y _z) (Math|Vector|BreakVector FireLine))
  (bind _weapondata (Variables|Default|GetWeaponData))
  (bind _weapondata_2 (Variables|Default|GetWeaponData))
  (bind _bulletspreadrangey (Variables|/Game/Blueprints/Data/DataAssets/Weapons/PDA_WeaponData.PDA_WeaponData_C|GetBulletSpreadRangeY _weapondata_2))
  (bind _bulletspreadrangez (Variables|/Game/Blueprints/Data/DataAssets/Weapons/PDA_WeaponData.PDA_WeaponData_C|GetBulletSpreadRangeZ _weapondata))
  (LocalVariables|SetXAxis _x)
  (LocalVariables|SetYAxis _y)
  (LocalVariables|SetZAxis _z)
  (return (Math|Vector|MakeVector (LocalVariables|GetXAxis) (+ (LocalVariables|GetYAxis) (* (Math|Random|RandomFloatinRange (* _bulletspreadrangey -1.0) _bulletspreadrangey) (Variables|Parameters|GetSpreadMultiplier))) (+ (LocalVariables|GetZAxis) (* (Math|Random|RandomFloatinRange (* _bulletspreadrangez -1.0) _bulletspreadrangez) (Variables|Parameters|GetSpreadMultiplier))))))

(fn ApplyDamage
  (params (DamagedActor :type Actor%20Object%20Reference) (HitInfo :type Hit%20Result%20Structure%20%28by%20ref%29) (HitFromDirection :type Vector%20%28by%20ref%29))
  (bind _returnvalue (Game|Damage|ApplyPointDamage DamagedActor (Variables|/Game/Blueprints/Data/DataAssets/Weapons/PDA_WeaponData.PDA_WeaponData_C|GetDamage (Variables|Default|GetWeaponData)) HitFromDirection HitInfo (Game|GetInstigatorController) self "/Script/Engine.DamageType"))
  (return _returnvalue))

(fn CalcutateRecoil
  (params (TimelineDirection :type ETimelineDirection%20Enum :default "Forward") (Interpolation :type Float%20%28double-precision%29))
  (bind _weapondata (Variables|Default|GetWeaponData))
  (bind _recoilforcex (Variables|/Game/Blueprints/Data/DataAssets/Weapons/PDA_WeaponData.PDA_WeaponData_C|GetRecoilForceX _weapondata))
  (LocalVariables|SetPlayerCharacter (Game|GetPlayerCharacter 0))
  (switch Utilities|FlowControl|Switch|SwitchonETimelineDirection TimelineDirection
    (:Forward
      (Pawn|Input|AddControllerPitchInput (LocalVariables|GetPlayerCharacter) (Math|Float|Lerp 0.0 (Variables|/Game/Blueprints/Data/DataAssets/Weapons/PDA_WeaponData.PDA_WeaponData_C|GetRecoilForceY (Variables|Default|GetWeaponData)) Interpolation))
      (Pawn|Input|AddControllerYawInput (LocalVariables|GetPlayerCharacter) (Math|Float|Lerp 0.0 (Math|Random|RandomFloatinRange (* _recoilforcex -1.0) _recoilforcex) Interpolation))
      (return))
    (:Backward
      (Pawn|Input|AddControllerPitchInput (LocalVariables|GetPlayerCharacter) (* (Math|Float|Lerp 0.0 (Variables|/Game/Blueprints/Data/DataAssets/Weapons/PDA_WeaponData.PDA_WeaponData_C|GetRecoilForceY (Variables|Default|GetWeaponData)) Interpolation) -1.1))
      (return))))

(fn SpawnProjectile
  (params (IsHit :type Boolean) (ImpactPoint :type Vector) (TraceEnd :type Vector))
  (bind _projectilespawnlocation (Variables|Default|GetProjectileSpawnLocation))
  (bind _returnvalue (Transformation|GetWorldLocation _projectilespawnlocation))
  (Game|SpawnActorfromClass "/Game/Blueprints/Actors/Projectiles/BP_ProjectileBase.BP_ProjectileBase_C" (Math|Transform|MakeTransform _returnvalue (Math|Rotator|FindLookatRotation _returnvalue (select IsHit ImpactPoint TraceEnd)) (Transformation|GetWorldScale (Variables|Default|GetProjectileSpawnLocation))) "AlwaysSpawn" "MultiplyWithRoot" 0 (Variables|/Game/Blueprints/Data/DataAssets/Weapons/PDA_WeaponData.PDA_WeaponData_C|GetProjectileSpeed (Variables|Default|GetWeaponData)) (Game|GetPlayerCharacter 0))
  (return))

(fn CastTrace
  (bind _output_get (LocalVariables|SetCameraLocation (Transformation|GetWorldLocation (Variables|Parameters|GetStartLineLocation))))
  (bind _spreadfireline (Firing|SpreadBullet (+ _output_get (* (Math|Vector|GetForwardVector (Transformation|GetWorldRotation (Variables|Parameters|GetStartLineLocation))) (Variables|/Game/Blueprints/Data/DataAssets/Weapons/PDA_WeaponData.PDA_WeaponData_C|GetRange (Variables|Default|GetWeaponData))))))
  (bind (_outhit _returnvalue) (Collision|LineTraceByChannel (LocalVariables|GetCameraLocation) _spreadfireline "TraceTypeQuery1" false (Utilities|Array|MakeArray (Game|GetPlayerCharacter 0)) "None"))
  (LocalVariables|SetHitResultInfo _outhit)
  (LocalVariables|SetIsTraceHit _returnvalue)
  (Firing|ApplyDamage (.HitActor (Collision|BreakHitResult (LocalVariables|GetHitResultInfo))) (LocalVariables|GetHitResultInfo) (Math|Vector|GetForwardVector (Variables|Default|GetProjectileSpawnLocation)))
  (return (LocalVariables|GetIsTraceHit) (.ImpactPoint (Collision|BreakHitResult (LocalVariables|GetHitResultInfo))) (.TraceEnd (Collision|BreakHitResult (LocalVariables|GetHitResultInfo)))))

(fn Fire
  (if (Ammo|CheckAmmoCount)
    (Ammo|DecrementAmmo)
    (Firing|ShakeCamera)
    (Firing|SpawnMuzzleFlash)
    (CallFunction|ApplyRecoil)
    (CallFunction|ShowMuzzleLight)
    (Sound|PlayShotSound)
    (for _index (range 1 (Variables|/Game/Blueprints/Data/DataAssets/Weapons/PDA_WeaponData.PDA_WeaponData_C|GetProjectilesPerShot (Variables|Default|GetWeaponData)))
      (bind (_ishit _impactpoint _traceend) (Firing|CastTrace))
      (Firing|SpawnProjectile _ishit _impactpoint _traceend))
    (Default|CallOnFire)
    (CallFunction|EndShot)
    (return)
    (else
      (Sound|PlayEmptySound)
      (return))))

(fn CheckAmmoCount
  (return (< 0 (Variables|Parameters|GetCurrentAmmo))))

(fn DecrementAmmo
  (bind _result (Math|Integer|DecrementInt (Variables|Parameters|GetCurrentAmmo))
    (:%20%20
      (Variables|Parameters|SetCurrentAmmo (Math|Integer|Clamp(Integer) _result 0 (Variables|/Game/Blueprints/Data/DataAssets/Weapons/PDA_WeaponData.PDA_WeaponData_C|GetMaxAmmo (Variables|Default|GetWeaponData))))
      (return))))

(fn ShakeCamera
  (CameraShakes|StartCameraShake (Game|GetPlayerCameraManager 0) (Variables|/Game/Blueprints/Data/DataAssets/Weapons/PDA_WeaponData.PDA_WeaponData_C|GetCameraShake (Variables|Default|GetWeaponData)) (Variables|/Game/Blueprints/Data/DataAssets/Weapons/PDA_WeaponData.PDA_WeaponData_C|GetCameraShakeScale (Variables|Default|GetWeaponData)) "CameraLocal" "0, 0, 0")
  (return))

(fn InitializeWeapon
  (params (WeaponData :type PDA%20Weapon%20Data%20Object%20Reference) (CurrentAmmo :type Integer))
  (bind _output_get (Variables|Default|SetWeaponData WeaponData))
  (Components|StaticMesh|SetStaticMesh (Variables|Default|GetWeaponMesh) (Variables|/Game/Blueprints/Data/DataAssets/Weapons/PDA_WeaponData.PDA_WeaponData_C|GetWeaponStaticMesh _output_get))
  (Ammo|SetAmmoCount CurrentAmmo)
  (WeaponManagment|EnableWeapon)
  (return))

(fn GetWeaponData
  (bind _weapondata (Variables|Default|GetWeaponData)
    (:then
      (return _weapondata))
    (:else
      (Development|PrintString "Data isn't Valid!"))))

(fn DisableWeapon
  (Variables|Default|SetIsEnable false)
  (Timers|ClearTimers)
  (WeaponManagment|StopTimelines)
  (CallFunction|OnDisableWeapon)
  (return))

(fn EnableWeapon
  (Variables|Default|SetIsEnable true)
  (CallFunction|OnEnableWeapon)
  (WeaponManagment|UpdateWeapon)
  (return))

(fn SetTimerforUnlockBurstMode
  (bind _returnvalue (Utilities|Time|SetTimerbyEvent (EventDispatchers|CreateEvent :!event Custom|UnlockBurstMode) (Variables|/Game/Blueprints/Data/DataAssets/Weapons/PDA_WeaponData.PDA_WeaponData_C|GetBurstLockTime (Variables|Default|GetWeaponData))))
  (Variables|Timers|SetUnlockBurstMode_TimerHandle _returnvalue)
  (return))

(fn SetTimerforUnlockFire
  (params (OnEnabledWeapon :type Boolean))
  (LocalVariables|SetTime (Math|Float|SelectFloat (Variables|Default|GetWeaponPrepareTime) (Variables|/Game/Blueprints/Data/DataAssets/Weapons/PDA_WeaponData.PDA_WeaponData_C|GetFireRate (Variables|Default|GetWeaponData)) OnEnabledWeapon))
  (bind _returnvalue (Utilities|Time|SetTimerbyEvent (EventDispatchers|CreateEvent :!event Custom|UnlockFire) (LocalVariables|GetTime)))
  (Variables|Timers|SetEnableFire_TimerHandle _returnvalue)
  (return))

(fn SetTimerforStartBurstMode
  (bind _returnvalue (Utilities|Time|SetTimerbyEvent (EventDispatchers|CreateEvent :!event Custom|BurstMode) (Variables|/Game/Blueprints/Data/DataAssets/Weapons/PDA_WeaponData.PDA_WeaponData_C|GetFireRate (Variables|Default|GetWeaponData)) true))
  (Variables|Timers|SetStartBurstMode_TimerHandle _returnvalue)
  (return))

(fn PlayShotSound
  (Audio|PlaySoundatLocation (Variables|/Game/Blueprints/Data/DataAssets/Weapons/PDA_WeaponData.PDA_WeaponData_C|GetShotSound (Variables|Default|GetWeaponData)) (Transformation|GetWorldLocation (Variables|Default|GetProjectileSpawnLocation)) "0, 0, 0" 1.0 1.0 0.0 0 0 0 0)
  (return))

(fn ReloadWeapon
  (Timers|ClearTimers)
  (CallFunction|OnReload)
  (CallFunction|OnDisableWeapon))

(fn SpawnMuzzleFlash
  (Niagara|SpawnSystemAttached (Variables|/Game/Blueprints/Data/DataAssets/Weapons/PDA_WeaponData.PDA_WeaponData_C|GetMuzzleFlash (Variables|Default|GetWeaponData)) (Variables|Default|GetMuzzleFlashLocation) "None" "0, 0, 0" "0, 0, 0" "KeepRelativeOffset" true)
  (return))

(fn ClearTimers
  (Utilities|Time|ClearandInvalidateTimerbyHandle (Variables|Timers|GetEnableFire_TimerHandle))
  (Utilities|Time|ClearandInvalidateTimerbyHandle (Variables|Timers|GetUnlockBurstMode_TimerHandle))
  (Utilities|Time|ClearandInvalidateTimerbyHandle (Variables|Timers|GetStartBurstMode_TimerHandle))
  (return))

(fn StopTimelines
  (Audio|Components|Audio|Stop (Variables|Default|GetRecoilMovement_Timeline))
  (Audio|Components|Audio|Stop (Variables|Default|GetMuzzleLight_Timeline))
  (Audio|Components|Audio|Stop (Variables|Default|GetReload_Timeline))
  (return))

(fn UpdateWeapon
  (Default|CallOnUpdateWeapon (Variables|Parameters|GetCurrentAmmo))
  (return))

(fn SetSpreadMultiplier
  (params (Multiplier :type Float%20%28double-precision%29))
  (Variables|Parameters|SetSpreadMultiplier Multiplier)
  (return))

(fn PlayReloadSound
  (Audio|PlaySoundatLocation (Variables|/Game/Blueprints/Data/DataAssets/Weapons/PDA_WeaponData.PDA_WeaponData_C|GetReloadSound (Variables|Default|GetWeaponData)) (Transformation|GetWorldLocation (Variables|Default|GetProjectileSpawnLocation)) "0, 0, 0" 1.0 1.0 0.0 0 0 0 0)
  (return))

(fn PlayEmptySound
  (Variables|Default|GetEmptySoundInstance
    (:then)
    (:else
      (bind _returnvalue (Audio|SpawnSoundatLocation (Variables|Default|GetEmptyMagazineSound) (Transformation|GetWorldLocation (Variables|Default|GetProjectileSpawnLocation)) "0, 0, 0" 1.0 1.0 0.0 0 0))
      (Variables|Default|SetEmptySoundInstance _returnvalue)
      (return))))