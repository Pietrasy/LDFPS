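; Weapon pickup spawner, built on a parent item class, that displays a weapon and offers it to the player character.
; On BeginPlay it async-loads a weapon data asset to set mesh, name, description and full ammo before calling the parent BeginPlay.
; Execute messages the player with the weapon data and itself.
; DropWeapon swaps in a given weapon and ammo count, refreshes mesh and text, and plays the pickup sound.
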(event EventBeginPlay
  ;[0.15 0.15 0.15 0.5] Async load weapon data asset
  (bind _object (Utilities|AsyncLoadAsset (Variables|Default|GetWeaponData))
    (:Completed
      (bind _aspda_weapon_data (Utilities|Casting|CastToPDA_WeaponData _object))
      (Variables|Default|SetWeaponDataAsset _aspda_weapon_data)
      (Components|StaticMesh|SetStaticMesh (Variables|Default|GetItemStaticMesh) (Variables|/Game/Blueprints/Data/DataAssets/Weapons/PDA_WeaponData.PDA_WeaponData_C|GetWeaponStaticMesh (Variables|Default|GetWeaponDataAsset))) ; Set static mesh to mesh from data asset
      ;[0.15 0.15 0.15 0.5] Set text and description to displays by spawner
      (Variables|Default|SetItemName (Variables|/Game/Blueprints/Data/DataAssets/Weapons/PDA_WeaponData.PDA_WeaponData_C|GetName (Variables|Default|GetWeaponDataAsset)))
      (Variables|Default|SetItemDescription (Variables|/Game/Blueprints/Data/DataAssets/Weapons/PDA_WeaponData.PDA_WeaponData_C|GetDescription (Variables|Default|GetWeaponDataAsset)))
      (Variables|Default|SetCurrentAmmo (Variables|/Game/Blueprints/Data/DataAssets/Weapons/PDA_WeaponData.PDA_WeaponData_C|GetMaxAmmo (Variables|Default|GetWeaponDataAsset))) ; New spawns weapon will be full ammo
      (|CallParentFunction))))

(event EventDropWeapon
  (params (WeaponData :type PDA%20Weapon%20Data%20Object%20Reference) (CurrentAmmo :type Integer))
  (CallFunction|SetNewWeapon WeaponData CurrentAmmo)
  (CallFunction|PlayPickupSound))

(fn ConstructionScript
  (|CallParentFunction))

(fn Execute
  (params (PlayerCharacter :type Object%20Object%20Reference))
  (|CallParentFunction PlayerCharacter)
  (bind _candestroy (Class|BPIInteractions|PickupWeapon(Message) PlayerCharacter (Variables|Default|GetWeaponDataAsset) self))
  (return _candestroy))

(fn ReturnCurrentAmmo
  (return (Variables|Default|GetCurrentAmmo)))

(fn SetWidgetsText
  ;[0.15 0.15 0.15 0.5] Set text and description to displays by spawner
  (Variables|Default|SetItemName (Variables|/Game/Blueprints/Data/DataAssets/Weapons/PDA_WeaponData.PDA_WeaponData_C|GetName (Variables|Default|GetWeaponDataAsset)))
  (Variables|Default|SetItemDescription (Variables|/Game/Blueprints/Data/DataAssets/Weapons/PDA_WeaponData.PDA_WeaponData_C|GetDescription (Variables|Default|GetWeaponDataAsset)))
  (|CallParentFunction))

(fn SetNewWeapon
  (params (NewWeaponData :type PDA%20Weapon%20Data%20Object%20Reference) (CurrentAmmo :type Integer))
  (Variables|Default|SetWeaponDataAsset NewWeaponData)
  (Variables|Default|SetCurrentAmmo CurrentAmmo)
  (Components|StaticMesh|SetStaticMesh (Variables|Default|GetItemStaticMesh) (Variables|/Game/Blueprints/Data/DataAssets/Weapons/PDA_WeaponData.PDA_WeaponData_C|GetWeaponStaticMesh NewWeaponData))
  (CallFunction|SetWidgetsText)
  (return))