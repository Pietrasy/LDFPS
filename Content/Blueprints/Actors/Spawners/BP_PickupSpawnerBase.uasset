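; Base pickup actor that spins its item mesh through a timeline and shows name, description and "E" button widgets.
; Any overlap with its radius sphere reveals the enabled widgets with animations, and leaving collapses them.
; Interact calls Execute, a stub returning true that children can override; on success it plays a sound and destroys the actor.
; ReturnCurrentAmmo is also a stub, returning zero.
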(event OnComponentBeginOverlap(RadiusSphere)
  (params (OverlappedComponent :type Primitive%20Component%20Object%20Reference) (OtherActor :type Actor%20Object%20Reference) (OtherComp :type Primitive%20Component%20Object%20Reference) (OtherBodyIndex :type Integer) (bFromSweep :type Boolean) (SweepResult :type Hit%20Result%20Structure%20%28by%20ref%29))
  (Widget|ShowWidgets)
  (Widget|PlayWidgetsAnimation))

(event OnComponentEndOverlap(RadiusSphere)
  (params (OverlappedComponent :type Primitive%20Component%20Object%20Reference) (OtherActor :type Actor%20Object%20Reference) (OtherComp :type Primitive%20Component%20Object%20Reference) (OtherBodyIndex :type Integer))
  (Widget|CollapseWidgets)
  (Widget|StopWidgetsAnimation))

(event Custom|PickupRotation
  (bind _interpolation (Timeline|PickupRotation_Timeline PlayFromStart)
    (:Update
      (bind _output_get (Variables|MeshRotation|SetCurrentStaticMeshRotation (* _interpolation 3.6e+02)))
      (bind _output_get_2 (Variables|MeshRotation|SetDeltaRotation (- _output_get (Variables|MeshRotation|GetPreviousStaticMeshRotation))))
      (Transformation|AddRelativeRotation (Variables|Default|GetItemStaticMesh) (Math|Rotator|MakeRotator 0.0 0.0 _output_get_2) false false)
      (Variables|MeshRotation|SetPreviousStaticMeshRotation (Variables|MeshRotation|GetCurrentStaticMeshRotation)))))

(event EventBeginPlay
  (Widget|CacheWidgets)
  (CallFunction|PickupRotation)
  (CallFunction|SetWidgetsText))

(event EventInteract
  (params (Interactor :type Actor%20Object%20Reference))
  (bind _issuccess (CallFunction|Execute Interactor))
  (if _issuccess
    (CallFunction|PlayPickupSound)
    (Widget|CollapseWidgets)
    (Widget|StopWidgetsAnimation)
    (Actor|DestroyActor)))

(fn ConstructionScript)

(fn CacheWidgets
  (bind _aswbp_item_info (Utilities|Casting|CastToWBP_ItemInfo (UserInterface|GetWidget (Variables|Default|GetInfoWidgetComponent))))
  (Variables|Widget|SetInfoWidget _aswbp_item_info)
  (bind _aswbp_item_name (Utilities|Casting|CastToWBP_ItemName (UserInterface|GetWidget (Variables|Default|GetNameWidgetComponent))))
  (Variables|Widget|SetNameWidget _aswbp_item_name)
  (bind _aswbp_interaction_button (Utilities|Casting|CastToWBP_InteractionButton (UserInterface|GetWidget (Variables|Default|GetPickupButtonWidgetComponent))))
  (Variables|Widget|SetPickupWidget _aswbp_interaction_button)
  (return))

(fn ShowWidgets
  (Widget|ShowInfoWidgets)
  (Widget|ShowNameWidgets)
  (Widget|ShowButtonWidgets)
  (return))

(fn CollapseWidgets
  (Widget|SetVisibility (Variables|Widget|GetInfoWidget) "Collapsed")
  (Widget|SetVisibility (Variables|Widget|GetNameWidget) "Collapsed")
  (Widget|SetVisibility (Variables|Widget|GetPickupWidget) "Collapsed")
  (return))

(fn PlayWidgetsAnimation
  (bind _infowidget (Variables|Widget|GetInfoWidget))
  (bind _namewidget (Variables|Widget|GetNameWidget))
  (bind _pickupwidget (Variables|Widget|GetPickupWidget))
  (bind _pickupwidget_2 (Variables|Widget|GetPickupWidget))
  (UserInterface|Animation|PlayAnimation _infowidget (Variables|/Game/Blueprints/Widgets/InteractionWidgets/WBP_ItemInfo.WBP_ItemInfo_C|GetAppear _infowidget) 0.0 1 "Forward" 1.0 false)
  (UserInterface|Animation|PlayAnimation _namewidget (Variables|/Game/Blueprints/Widgets/InteractionWidgets/WBP_ItemName.WBP_ItemName_C|GetAppear _namewidget) 0.0 1 "Forward" 1.0 false)
  (UserInterface|Animation|PlayAnimation _pickupwidget_2 (Variables|/Game/Blueprints/Widgets/InteractionWidgets/WBP_InteractionButton.WBP_InteractionButton_C|GetAppear _pickupwidget_2) 0.0 1 "Forward" 1.0 false)
  (UserInterface|Animation|PlayAnimation _pickupwidget (Variables|/Game/Blueprints/Widgets/InteractionWidgets/WBP_InteractionButton.WBP_InteractionButton_C|GetBouncing_Loop _pickupwidget) 0.0 0 "Forward" 1.0 false)
  (return))

(fn StopWidgetsAnimation
  (Class|UserWidget|StopAllAnimations (Variables|Widget|GetInfoWidget))
  (Class|UserWidget|StopAllAnimations (Variables|Widget|GetNameWidget))
  (Class|UserWidget|StopAllAnimations (Variables|Widget|GetPickupWidget))
  (return))

(fn ShowInfoWidgets
  (if (Variables|Widget|GetIsInfoDisplay)
    (Widget|SetVisibility (Variables|Widget|GetInfoWidget) "Visible")
    (return)))

(fn ShowNameWidgets
  (if (Variables|Widget|GetIsNameDisplay)
    (Widget|SetVisibility (Variables|Widget|GetNameWidget) "Visible")
    (return)))

(fn ShowButtonWidgets
  (if (Variables|Widget|GetIsButtonDisplay)
    (Widget|SetVisibility (Variables|Widget|GetPickupWidget) "Visible")
    (return)))

(fn Execute
  (params (PlayerCharacter :type Object%20Object%20Reference))
  (return true))

(fn SetWidgetsText
  (Default|SetText (Variables|Widget|GetNameWidget) (Variables|Default|GetItemName))
  (Default|SetText (Variables|Widget|GetInfoWidget) (Variables|Default|GetItemDescription))
  (Default|SetText (Variables|Widget|GetPickupWidget) "E")
  (return))

(fn PlayPickupSound
  (Audio|PlaySoundatLocation (Variables|Default|GetPickupSound) (Transformation|GetActorLocation) "0, 0, 0" 1.0 1.0 0.0 0 0 0 0)
  (return))

(fn ReturnCurrentAmmo
  (return 0))