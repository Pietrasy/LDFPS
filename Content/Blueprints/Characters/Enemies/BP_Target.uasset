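; Shootable target enemy that goes down when hit and becomes active again after a random delay.
; Point damage counts only from the front, tested by a dot product of hit normal and forward vector; radial damage always counts.
; A valid hit shows the instigator's hitmarker and calls OnDeath, disabling damage and capsule collision and starting the get-up timer.
; GetUp restores both.
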(event Custom|OnDeath
  (Variables|Actor|SetbCanBeDamaged false)
  (Collision|SetCollisionEnabled (Variables|Default|GetCapsuleCollision) "NoCollision")
  (Timers|SetTimerforGetUp))

(event Custom|GetUp
  (Collision|SetCollisionEnabled (Variables|Default|GetCapsuleCollision) "QueryAndPhysics")
  (Variables|Actor|SetbCanBeDamaged true))

(event Game|Damage|EventPointDamage
  (params (Damage :type Float%20%28single-precision%29) (DamageType :type Damage%20Type%20Object%20Reference) (HitLocation :type Vector :default "0, 0, 0") (HitNormal :type Vector :default "0, 0, 0") (HitComponent :type Primitive%20Component%20Object%20Reference) (BoneName :type Name :default "None") (ShotFromDirection :type Vector :default "0, 0, 0") (InstigatedBy :type Controller%20Object%20Reference) (DamageCauser :type Actor%20Object%20Reference) (HitInfo :type Hit%20Result%20Structure%20%28by%20ref%29))
  ;[0.15 0.15 0.15 0.5] Handle applied damages
  (bind _isfront (Damage|CheckWhetherHitCamefromFront HitNormal))
  (Damage|RespondtoDamage _isfront InstigatedBy))

(event Game|Damage|EventRadialDamage
  (params (DamageReceived :type Float%20%28single-precision%29) (DamageType :type Damage%20Type%20Object%20Reference) (Origin :type Vector :default "0, 0, 0") (HitInfo :type Hit%20Result%20Structure%20%28by%20ref%29) (InstigatedBy :type Controller%20Object%20Reference) (DamageCauser :type Actor%20Object%20Reference))
  ;[0.15 0.15 0.15 0.5] Handle applied damages
  (Damage|RespondtoDamage true InstigatedBy))

(fn ConstructionScript)

(fn RespondtoDamage
  (params (IsHit :type Boolean) (Instigator :type Controller%20Object%20Reference))
  (if IsHit
    (Class|BPIHitmarkerNotify|ShowHitmarker(Message) Instigator)
    (CallFunction|OnDeath)
    (return)
    (else
      (return))))

(fn CheckWhetherHitCamefromFront
  (params (HitNormal :type Vector))
  (return (< 0.16 (Math|Vector|DotProduct HitNormal (Transformation|GetActorForwardVector)))))

(fn SetTimerforGetUp
  (bind _returnvalue (Utilities|Time|SetTimerbyEvent (EventDispatchers|CreateEvent :!event Custom|GetUp) (Math|Random|RandomFloatinRange (Variables|Default|GetMinTimeToGetUp) (Variables|Default|GetMaxTimeToGetUp))))
  (Variables|Timers|SetGetUp_TimerHandle _returnvalue)
  (return))