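; BP_Player is the first-person player character Blueprint, handling running, weapon pickup and fire feedback.
; It broadcasts an initialization dispatcher on BeginPlay and plays a recoil montage on the arm mesh when a weapon fires.
; Running toggles switch the max walk speed and broadcast a speed-change dispatcher, while a separate setter tracks movement state.
; Weapon pickup is delegated to BPWeaponComponent, which is also exposed through a getter.
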(event Custom|OnWeaponFire
  (Animation|Montage|PlayMontage (Variables|Default|GetArmSkeletalMesh) "/Game/Art/Animations/Players/AM_FirstPerson_Recoil_Large.AM_FirstPerson_Recoil_Large"))

(event EventBeginPlay
  (Default|CallOnCharacterInitialization))

(fn ConstructionScript
  (|CallParentFunction))

(fn ToogleRunning
  (params (IsRunning :type Boolean))
  (if IsRunning
    (Variables|/Script/Engine.CharacterMovementComponent|SetMaxWalkSpeed (Variables|Character|GetCharacterMovement) 9e+02)
    (Variables|Movement|SetIsRunning true)
    (else
      (Variables|/Script/Engine.CharacterMovementComponent|SetMaxWalkSpeed (Variables|Character|GetCharacterMovement) 6e+02)
      (Variables|Movement|SetIsRunning false)))
  (Default|CallOnChangeSpeed)
  (return))

(fn SetMovementState
  (params (IsMoving :type Boolean))
  (Variables|Movement|SetIsMoving IsMoving)
  (return))

(fn PickupWeapon
  (params (WeaponData :type PDA%20Weapon%20Data%20Object%20Reference) (PickupSpawner :type Object%20Object%20Reference))
  (bind _isspawnertobedestroyed (Default|PickupWeapon (Variables|Default|GetBP_WeaponComponent) WeaponData PickupSpawner))
  (return _isspawnertobedestroyed))

(fn ReturnWeaponComponent
  (return (Variables|Default|GetBP_WeaponComponent)))